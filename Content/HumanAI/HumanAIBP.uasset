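; HumanAIBP is an armed human AI character that spawns a gun attached to its hand socket on BeginPlay and caches the player character.
; StartShooting and StopShooting toggle a flag that Tick-driven Shoot checks, with a Delay pacing the shots.
; Each shot runs a forward debug line trace and spawns a ProjectileTrace actor from the hand.
; The trace's player-hit check leads nowhere, as the health decrement is disconnected.
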(event Custom|StartShooting
  (Variables|Default|SetIsShooting true))

(event Custom|StopShooting
  (Variables|Default|SetIsShooting false))

(event Custom|Shoot
  (if (Variables|Default|GetIsShooting)
    (Utilities|FlowControl|Delay 0.2)
    (bind _outhit (Collision|LineTraceByChannel (+ (Transformation|GetSocketLocation (Variables|Character|GetMesh) "InHand") (* (Math|Vector|GetForwardVector (Transformation|GetActorRotation)) 75.0)) (+ (Transformation|GetActorLocation) (* (Math|Vector|GetForwardVector (Transformation|GetActorRotation)) 2e+03)) "TraceTypeQuery3" false 0 "ForDuration"))
    (Game|SpawnActorfromClass "/Game/Levels/ChapterOne/Effects/ProjectileTrace.ProjectileTrace_C" (Math|Transform|MakeTransform (Transformation|GetSocketLocation (Variables|Character|GetMesh) "InHand") (Transformation|GetActorRotation)) "Undefined" 0 0)
    (if (== (.HitActor (Collision|BreakHitResult _outhit)) (Variables|Default|GetPlayerRef))
      _)))

(event EventBeginPlay
  (bind _asthird_person_character (Utilities|Casting|CastToThirdPersonCharacter (Game|GetPlayerCharacter 0)))
  (Variables|Default|SetPlayerRef _asthird_person_character)
  (bind _returnvalue (Game|SpawnActorfromClass "/Game/HumanAI/HumanAIGun.HumanAIGun_C" (Transformation|GetSocketTransform (Variables|Character|GetMesh) "InHand" "RTS_World") "Undefined" 0 0))
  (Transformation|AttachComponentToComponent _returnvalue (Variables|Character|GetMesh) "InHand" "SnapToTarget" "SnapToTarget" "SnapToTarget" true))

(event EventTick
  (params (DeltaSeconds :type Float%20%28single-precision%29))
  (CallFunction|Shoot))

(fn ConstructionScript)