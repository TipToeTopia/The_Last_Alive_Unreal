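; Zombie enemy character that attacks the player, can be killed by damage or stealth takedown, and spawns a random ammo pickup on death.
; While alive, Tick drives a sight-detection widget; once dead, it hides the widget and attempts the drop once.
; Attack plays an animation and directly subtracts player health.
; A box overlap enables takedowns, and both death paths set the AI blackboard flag, disable movement and collision, then destroy the actor.
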(event OnComponentBeginOverlap(TakeDownBoxCollision)
  (params (OverlappedComponent :type Primitive%20Component%20Object%20Reference) (OtherActor :type Actor%20Object%20Reference) (OtherComp :type Primitive%20Component%20Object%20Reference) (OtherBodyIndex :type Integer) (bFromSweep :type Boolean) (SweepResult :type Hit%20Result%20Structure%20%28by%20ref%29))
  ;[1 1 1] Stealth Collision Enter/ Exit boxes
  (bind _asthird_person_character (Utilities|Casting|CastToThirdPersonCharacter OtherActor))
  (Variables|/Game/ThirdPersonBP/Blueprints/ThirdPersonCharacter.ThirdPersonCharacter_C|SetCanTakeDown? _asthird_person_character true))

(event OnComponentEndOverlap(TakeDownBoxCollision)
  (params (OverlappedComponent :type Primitive%20Component%20Object%20Reference) (OtherActor :type Actor%20Object%20Reference) (OtherComp :type Primitive%20Component%20Object%20Reference) (OtherBodyIndex :type Integer))
  ;[1 1 1] Stealth Collision Enter/ Exit boxes
  (bind _asthird_person_character (Utilities|Casting|CastToThirdPersonCharacter OtherActor))
  (Variables|/Game/ThirdPersonBP/Blueprints/ThirdPersonCharacter.ThirdPersonCharacter_C|SetCanTakeDown? _asthird_person_character false))

(event Custom|Attack
  (bind _thirdpersoncharacter (Variables|Default|GetThirdPersonCharacter))
  ;[1 1 1] ATTACK
  (Components|Animation|PlayAnimation (Variables|Character|GetMesh) "/Game/Animations/ZombieAI/ZombieAttack_2_4UE4.ZombieAttack_2_4UE4" false)
  (bind _output_get (Variables|/Game/ThirdPersonBP/Blueprints/ThirdPersonCharacter.ThirdPersonCharacter_C|SetPlayerHealth _thirdpersoncharacter (- (Variables|/Game/ThirdPersonBP/Blueprints/ThirdPersonCharacter.ThirdPersonCharacter_C|GetPlayerHealth _thirdpersoncharacter) (Variables|/Game/ThirdPersonBP/Blueprints/ThirdPersonCharacter.ThirdPersonCharacter_C|GetZombieDamage _thirdpersoncharacter))))
  (Utilities|FlowControl|Delay 1.5)
  (Components|Animation|SetAnimationMode (Variables|Character|GetMesh) "AnimationBlueprint"))

(event Custom|TakeDown
  ;[1 1 1] ZombieStealth Death
  (bind _aszombie_aic (Utilities|Casting|CastToZombieAIC (Pawn|GetController)))
  (AI|Components|Blackboard|SetValueasBool (Variables|/Script/AIModule.AIController|GetBlackboard _aszombie_aic) (Utilities|Name|MakeLiteralName "IsDead?") true)
  (Pawn|Components|CharacterMovement|DisableMovement (Variables|Character|GetCharacterMovement))
  (Collision|SetActorEnableCollision false)
  (Animation|PlayAnimMontage "/Game/Animations/ZombieAI/Stealth_Assassination_A_Montage.Stealth_Assassination_A_Montage" 1.0 "None")
  (Variables|Default|SetIsZombieDead? true)
  (Variables|Default|SetHealth 0.0)
  (Utilities|FlowControl|Delay 6e+01)
  (Actor|DestroyActor))

(event EventBeginPlay
  (bind _assight_detection (Utilities|Casting|CastToSightDetection (UserInterface|GetUserWidgetObject (Variables|Default|GetDetection))))
  (Variables|Default|SetSightDetection _assight_detection)
  (Variables|/Game/AI/SightDetection.SightDetection_C|SetPawnOwner _assight_detection self)
  (bind _asthird_person_character (Utilities|Casting|CastToThirdPersonCharacter (Game|GetPlayerCharacter 0)))
  (Variables|Default|SetThirdPersonCharacter _asthird_person_character)
  (bind _aszombie_aic (Utilities|Casting|CastToZombieAIC (Pawn|GetController)))
  (Variables|Default|SetZombieAIC _aszombie_aic))

(event EventTick
  (params (DeltaSeconds :type Float%20%28single-precision%29))
  (if (Variables|Default|GetIsZombieDead?)
    ;[1 1 1] ZombieDead
    (Widget|SetVisibility (Variables|Default|GetSightDetection) "Hidden")
    (Utilities|FlowControl|DoOnce false
      (:Completed
        (Game|SpawnActorfromClass (Utilities|Select :Index (Math|Random|RandomInteger 5) :Option%200 "/Game/Levels/ChapterOne/Guns/AmmoPickUps/ShotgunAmmo.ShotgunAmmo_C" :Option%201 "/Game/Levels/ChapterOne/Guns/AmmoPickUps/RifleAmmo.RifleAmmo_C" :Option%202 "/Game/Levels/ChapterOne/Guns/AmmoPickUps/PistolAmmo.PistolAmmo_C") (Transformation|GetActorTransform) "Undefined" 0 0)))
    (else
      (Default|ZombieSight (stale EventBeginPlay _assight_detection)))))

(event EventDoDamage
  (params (Damage :type Float%20%28single-precision%29) (HitResult :type Hit%20Result%20Structure))
  ;[1 1 1] Damage AND Death
  (Variables|Default|SetHealth (- (Variables|Default|GetHealth) Damage))
  (if (<= (- (Variables|Default|GetHealth) Damage) 0.0)
    (Variables|Default|SetIsZombieDead? true)
    (Utilities|FlowControl|Sequence
      (:then_0
        (bind _returnvalue (Animation|PlayAnimMontage "/Game/Animations/ZombieAI/Death_2_Montage.Death_2_Montage" 1.0 "None"))
        (bind _aszombie_aic (Utilities|Casting|CastToZombieAIC (Pawn|GetController)))
        (AI|Components|Blackboard|SetValueasBool (Variables|/Script/AIModule.AIController|GetBlackboard _aszombie_aic) (Utilities|Name|MakeLiteralName "IsDead?") true)
        (Pawn|Components|CharacterMovement|DisableMovement (Variables|Character|GetCharacterMovement))
        (Collision|SetActorEnableCollision false)
        (Utilities|FlowControl|Delay _returnvalue)
        (Actor|DestroyActor))
      (:then_1
        (Utilities|FlowControl|DoOnce false
          (:Completed
            (Audio|PlaySoundatLocation "/Game/Audio/AISound/ZombieAI/ZombieDeath.ZombieDeath" (Transformation|GetActorLocation) "0, 0, 0" 1.5 1.0 0.0 0 0 0)))))))

(fn ConstructionScript)